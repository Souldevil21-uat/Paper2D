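; A 2D sprite lift that travels between its origin and an end location, with its timeline rate set from a travel time.
; A timeline lerps the sprite position and, on finishing, waits for a stop delay before running the opposite way via LiftForward or LiftBackward.
; A character overlapping the safety collider mid-travel calls Play or Reverse on the timeline.
; The construction script applies the color and previews either endpoint.
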(event `self.ReceiveBeginPlay`
  (`TimelineComponent.SetPlayRate` (`self.LiftTimeline`) (/ 1.0 (`self.TravelTimeInSeconds`)))
  (set `self.TestEndLocation` true))

(event `self.Safety Collider.OnComponentBeginOverlap`
  (params (OverlappedComponent :type "PrimitiveComponent Object Reference") (OtherActor :type "Actor Object Reference") (OtherComp :type "PrimitiveComponent Object Reference") (OtherBodyIndex :type Integer) (bFromSweep :type Boolean) (SweepResult :type "HitResult Structure (by ref)"))
  (bind _lifttimeline (`self.LiftTimeline`))
  (cast `/Game/Blueprints/MyCharacter` OtherActor)
  (if (`ActorComponent.IsActive` _lifttimeline)
    (if (`TimelineComponent.IsPlaying` _lifttimeline)
      (bind (_direction _newtrack_0) (`Timeline|LiftTimeline` :!label _label)
        (:`Update`
          (`SceneComponent.K2_SetRelativeLocation` (`self.Lift Sprite`) (`KismetMathLibrary.VLerp` (0.0 0.0 0.0) (`self.EndLocation`) _newtrack_0) false false))
        (:`Finished`
          (`KismetSystemLibrary.Delay` (`self.StopDelay`))
          (switch `ETimelineDirection` _direction
            (:`Forward`
              (`self.LiftBackward`))
            (:`Backward`
              (`self.LiftForward`)))))
      (else
        (goto _label :!via `Reverse`)))))

(event `LiftForward`
  (goto _label :!via `PlayFromStart`))

(event `LiftBackward`
  (goto _label :!via `ReverseFromEnd`))

(fn `UserConstructionScript`
  (bind _lift_sprite (`self.Lift Sprite`))
  (`SceneComponent.K2_SetRelativeLocation` _lift_sprite (`KismetMathLibrary.SelectVector` (`self.EndLocation`) (0.0 0.0 0.0) (`self.TestEndLocation`)) false false)
  (`PaperSpriteComponent.SetSpriteColor` _lift_sprite (`self.LiftColor`)))